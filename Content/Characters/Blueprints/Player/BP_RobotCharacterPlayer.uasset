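; BP_RobotCharacterPlayer is the player robot character Blueprint, adding attack input and animation on top of its parent class.
; Pressing R calls the Attack override, which runs the parent attack and then triggers AttackAnim.
; AttackAnim plays AttackMontage, waits twice its returned duration, then stops AM_MainPlayerAttack, referenced directly rather than through the variable.
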(event Custom|AttackAnim
  (bind _returnvalue (Animation|PlayAnimMontage (Variables|Default|GetAttackMontage) 1.0 "None"))
  (Utilities|FlowControl|Delay (* 2 _returnvalue))
  (Animation|StopAnimMontage "/Game/Characters/Animations/AM_MainPlayerAttack.AM_MainPlayerAttack"))

(event EventBeginPlay
  (|CallParentFunction) ; This node is disabled and will not be called.\nDrag off pins to build functionality.
)

(event Collision|EventActorBeginOverlap
  (params (OtherActor :type Actor%20Object%20Reference))
  (|CallParentFunction OtherActor) ; This node is disabled and will not be called.\nDrag off pins to build functionality.
)

(event EventTick
  (params (DeltaSeconds :type Float%20%28single-precision%29))
  (|CallParentFunction DeltaSeconds) ; This node is disabled and will not be called.\nDrag off pins to build functionality.
)

(event Input|KeyboardEvents|R
  (params (Key :type Key%20Structure :default "None"))
  (:Pressed
    (CallFunction|Attack)))

(fn ConstructionScript
  (|CallParentFunction))

(fn Attack
  (|CallParentFunction)
  (CallFunction|AttackAnim))