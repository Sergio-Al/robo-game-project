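; Base player controller that teleports the controlled pawn to a clicked or tapped point in the world.
; SetDestination presses and first-finger touches trace the Visibility channel and feed the hit into TransportToLocation.
; It ignores BP_BaseEnv hits and points within MinClickDistance, otherwise placing the pawn slightly above the hit, rotated toward it.
; A navigation-based MoveToLocation function exists but is only called from unreachable nodes.
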(event Input|ActionEvents|InputActionSetDestination
  (params (Key :type Key%20Structure :default "None"))
  (:Pressed
    (CallFunction|TransporttoLocation (.HitResult (Game|Player|GetHitResultUnderCursorbyChannel "TraceTypeQuery1" true)))))

(event Input|TouchEvents|InputTouch
  (params (Location :type Vector) (FingerIndex :type ETouchIndex%20Enum))
  (:Pressed
    (if (Utilities|Enum|Equal(Enum) FingerIndex "Touch1")
      (CallFunction|TransporttoLocation (.HitResult (Class|PlayerController|GetHitResultUnderFingerbyChannel FingerIndex "TraceTypeQuery1" true))))))

(fn ConstructionScript)

(fn MovetoLocation
  (params (Hit :type Hit%20Result%20Structure))
  (bind _location (Collision|BreakHitResult Hit))
  (if (>= (Math|Vector|VectorLength (- (Transformation|GetActorLocation (Pawn|GetControlledPawn)) _location)) (Variables|Default|GetMinClickDistance))
    (AI|Navigation|SimpleMovetoLocation self _location)))

(fn TransporttoLocation
  (params (Hit :type Hit%20Result%20Structure))
  (bind _returnvalue (Pawn|GetControlledPawn))
  (bind (_bblockinghit _binitialoverlap _time _distance _location _impactpoint _normal _impactnormal _physmat _hitactor) (Collision|BreakHitResult Hit))
  (bind _returnvalue_2 (Transformation|GetActorLocation _returnvalue))
  (bind (_x _y _z) (Math|Vector|BreakVector _location))
  (bind _returnvalue_3 (+ _z 1e+02))
  (bind _returnvalue_4 (Math|Vector|MakeVector _x _y _returnvalue_3))
  (Utilities|Casting|CastToBP_BaseEnv _hitactor
    (:CastFailed
      (if (Utilities|IsValid _returnvalue)
        (if (> (Math|Vector|VectorLength (- _location _returnvalue_2)) (Variables|Default|GetMinClickDistance))
          (Transformation|SetActorLocationAndRotation _returnvalue _returnvalue_4 (Math|Rotator|FindLookatRotation _returnvalue_2 _returnvalue_4)))))))