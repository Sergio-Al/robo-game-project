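; Base game mode that runs wave-based levels of robot enemies, tracks the current score and loads the top score from the save game.
; StartLevel scales the enemy count by a difficulty multiplier and starts a looping timer that spawns robots at random spawn-point actors until none remain.
; RegisterEnemyDeath adds score and, once the wave is fully spawned and cleared, has the player character reset its widget counter with the between-level wait time.
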(event Custom|SpawnEnemyInLevel
  (CallFunction|SpawnEnemy))

(event Custom|EndLevel
  (bind _asbp_base_player_character (Utilities|Casting|CastToBP_BasePlayerCharacter (Game|GetPlayerCharacter 0)))
  (Utilities|IsValid _asbp_base_player_character
    (:Is%20Valid
      (Default|ResetWidgetCounter _asbp_base_player_character (Variables|Default|GetSecondsToWaitForLevel)))))

(event EventBeginPlay
  (bind _returnvalue (SaveGame|LoadGamefromSlot "PlayerGame" 1))
  (bind _asbp_general_save_game (Utilities|Casting|CastToBP_GeneralSaveGame _returnvalue))
  (Variables|Default|SetTopScore (Math|Conversions|ToFloat(Integer) (Variables|/Game/Characters/Blueprints/Utils/BP_GeneralSaveGame.BP_GeneralSaveGame_C|GetTopScore _asbp_general_save_game))))

(event EventTick
  (params (DeltaSeconds :type Float%20%28single-precision%29)))

(fn ConstructionScript)

(fn StartLevel
  (Math|Integer|IncrementInt (Variables|Default|GetCurrentLevel)
    (:%20%20
      (CallFunction|IncreaseLevelDifficulty)
      (Utilities|Time|SetTimerbyFunctionName 0 "SpawnEnemyInLevel" (Variables|Default|GetSpawnFrequency) true))))

(fn IncreaseLevelDifficulty
  (bind _output_get (Variables|Default|SetLevelDifficulty (Math|Float|Round (* (Variables|Default|GetLevelDifficulty) (Variables|Default|GetDifficultyMultiplier)))))
  (Variables|Default|SetEnemiesSpawnRemaining _output_get))

(fn SpawnEnemy
  (bind _output (CallFunction|GetRandomEnemySpawnPoint))
  (Utilities|IsValid _output
    (:Is%20Valid
      (bind _returnvalue (Game|SpawnActorfromClass "/Game/Characters/Blueprints/NPC/BP_RobotEnemy.BP_RobotEnemy_C" (Transformation|GetActorTransform _output) "Undefined" 0 0))
      (Utilities|IsValid _returnvalue
        (:Is%20Valid
          (Utilities|Array|Add (Variables|Default|GetEnemies) _returnvalue)
          (bind _result (Math|Integer|DecrementInt (Variables|Default|GetEnemiesSpawnRemaining))
            (:%20%20
              (if (== _result 0)
                (Utilities|Time|ClearTimerbyFunctionName 0 "SpawnEnemyInLevel")))))))))

(fn GetRandomEnemySpawnPoint
  (bind _outactors (Actor|GetAllActorsOfClass "/Game/Environment/Props/BP_EnemiesSpawnPoint.BP_EnemiesSpawnPoint_C"))
  (return (Utilities|Array|Get(acopy) _outactors (Math|Random|RandomIntegerinRange 0 (Utilities|Array|LastIndex _outactors)))))

(fn IsLevelComplete
  (return (and (== (Utilities|Array|Length (Variables|Default|GetEnemies)) 0) (== (Variables|Default|GetEnemiesSpawnRemaining) 0))))

(fn RegisterEnemyDeath
  (params (Enemy :type BP%20Base%20Enemy%20Object%20Reference%20%28by%20ref%29))
  (Utilities|Array|RemoveItem (Variables|Default|GetEnemies) Enemy)
  (Variables|Default|SetCurrentScore (+ (Variables|Default|GetCurrentScore) 1e+01))
  (if (CallFunction|IsLevelComplete)
    (Development|PrintString "ENDING LEVEL")
    (CallFunction|EndLevel)))

(fn GetCurrentScore
  (return (Variables|Default|GetCurrentScore)))

(fn GetTopScore
  (return (Variables|Default|GetTopScore)))