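; Base enemy character that chases the player and provides shared health, attack and death logic.
; From BeginPlay it loops AI move-to toward the player's location, pausing briefly after each success or failure while alive.
; Helpers check range and damage the player, while Attack is a print-only parent stub.
; AutoDamage triggers the player's attack, subtracts that player's hit damage and, at zero health, registers the death with the game mode and destroys the enemy.
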(event EventBeginPlay
  (bind _returnvalue (Game|GetPlayerCharacter 0))
  (bind _asbp_base_player_character (Utilities|Casting|CastToBP_BasePlayerCharacter (Game|GetPlayerCharacter 0)))
  (Variables|Default|SetMainPlayerReference _asbp_base_player_character)
  (if (CallFunction|IsAlive) :!label _label
    (if (Utilities|IsValid _returnvalue)
      (AI|AIMoveTo self (Transformation|GetActorLocation _returnvalue) 0 5.0 true
        (:OnSuccess
          _)
        (:OnFail
          _))
      (Utilities|FlowControl|Delay 2.0)
      (goto _label))))

(event Collision|EventActorBeginOverlap
  (params (OtherActor :type Actor%20Object%20Reference)))

(event EventTick
  (params (DeltaSeconds :type Float%20%28single-precision%29)))

(fn ConstructionScript)

(fn IsWithinAttackRange
  (return (< (Transformation|GetDistanceTo (Game|GetPlayerCharacter 0)) (Variables|Attack|GetAttackRange))))

(fn IsAlive
  (return (not (Variables|Default|GetbIsDead))))

(fn Attack
  (Development|PrintString "parentAttack"))

(fn AttackPlayer
  (bind _returnvalue (Game|GetPlayerCharacter 0))
  (if (CallFunction|IsAlive)
    (if (Utilities|IsValid _returnvalue)
      (Game|Damage|ApplyDamage _returnvalue (Variables|Attack|GetDamagePerHit) 0 0))))

(fn CanAttack
  (return (and (CallFunction|IsWithinAttackRange) (CallFunction|IsAlive))))

(fn AutoDamage
  (bind _mainplayerreference (Variables|Default|GetMainPlayerReference))
  (if (CallFunction|IsAlive)
    (Default|Attack _mainplayerreference)
    (bind _return (CallFunction|DecreaseHealth (Variables|/Game/Characters/Blueprints/Player/BP_BasePlayerCharacter.BP_BasePlayerCharacter_C|GetDamagePerHit _mainplayerreference)))
    (Development|PrintString (Utilities|String|ToString(Float) _return))
    (if (== _return 0.0)
      (Variables|Default|SetbIsDead true)
      (bind _asbp_base_game_mode (Utilities|Casting|CastToBP_BaseGameMode (Game|GetGameMode)))
      (Default|RegisterEnemyDeath _asbp_base_game_mode self)
      (Actor|DestroyActor))))

(fn DecreaseHealth
  (params (Damage :type Float%20%28single-precision%29))
  (bind _output_get (Variables|Default|SetHealth (Math|Float|Clamp(Float) (- (Variables|Default|GetHealth) Damage) 0.0 1e+02)))
  (return _output_get))