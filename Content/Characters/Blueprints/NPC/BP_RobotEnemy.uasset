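; BP_RobotEnemy is a robot enemy NPC that reacts to the player entering its proximity volumes.
; When MainPlayerReference overlaps AttackCollision or DamageCollision, a looping timer starts calling AutoDamage or AttackPlayer respectively, and leaving that volume clears it.
; Both functions are referenced by name and not defined in this graph, and the BeginPlay, ActorBeginOverlap and Tick events are disabled stubs.
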(event OnComponentBeginOverlap(AttackCollision)
  (params (OverlappedComponent :type Primitive%20Component%20Object%20Reference) (OtherActor :type Actor%20Object%20Reference) (OtherComp :type Primitive%20Component%20Object%20Reference) (OtherBodyIndex :type Integer) (bFromSweep :type Boolean) (SweepResult :type Hit%20Result%20Structure%20%28by%20ref%29))
  ;[1 1 1] AutoDamage
  (if (== OtherActor (Variables|Default|GetMainPlayerReference))
    (Utilities|Time|SetTimerbyFunctionName 0 "AutoDamage" 0.1 true)))

(event OnComponentEndOverlap(AttackCollision)
  (params (OverlappedComponent :type Primitive%20Component%20Object%20Reference) (OtherActor :type Actor%20Object%20Reference) (OtherComp :type Primitive%20Component%20Object%20Reference) (OtherBodyIndex :type Integer))
  ;[1 1 1] AutoDamage
  (if (== OtherActor (Variables|Default|GetMainPlayerReference))
    (Utilities|Time|ClearTimerbyFunctionName 0 "AutoDamage")))

(event OnComponentBeginOverlap(DamageCollision)
  (params (OverlappedComponent :type Primitive%20Component%20Object%20Reference) (OtherActor :type Actor%20Object%20Reference) (OtherComp :type Primitive%20Component%20Object%20Reference) (OtherBodyIndex :type Integer) (bFromSweep :type Boolean) (SweepResult :type Hit%20Result%20Structure%20%28by%20ref%29))
  ;[1 1 1] Damage Player if its too close
  (if (== OtherActor (Variables|Default|GetMainPlayerReference))
    (Utilities|Time|SetTimerbyFunctionName 0 "AttackPlayer" 0.1 true)))

(event OnComponentEndOverlap(DamageCollision)
  (params (OverlappedComponent :type Primitive%20Component%20Object%20Reference) (OtherActor :type Actor%20Object%20Reference) (OtherComp :type Primitive%20Component%20Object%20Reference) (OtherBodyIndex :type Integer))
  ;[1 1 1] Damage Player if its too close
  (if (== OtherActor (Variables|Default|GetMainPlayerReference))
    (Utilities|Time|ClearTimerbyFunctionName 0 "AttackPlayer")))

(event EventBeginPlay
  (|CallParentFunction) ; This node is disabled and will not be called.\nDrag off pins to build functionality.
)

(event Collision|EventActorBeginOverlap
  (params (OtherActor :type Actor%20Object%20Reference))
  (|CallParentFunction OtherActor) ; This node is disabled and will not be called.\nDrag off pins to build functionality.
)

(event EventTick
  (params (DeltaSeconds :type Float%20%28single-precision%29))
  (|CallParentFunction DeltaSeconds) ; This node is disabled and will not be called.\nDrag off pins to build functionality.
)

(fn ConstructionScript
  (|CallParentFunction))